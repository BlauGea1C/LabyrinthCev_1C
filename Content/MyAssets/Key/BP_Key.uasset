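; BP_Key is a key pickup that the player collects by pressing interact while it is overlapped.
; It enables input at BeginPlay and uses a Gate, opened and closed by unfiltered actor overlap events, to block IA_Interact from triggering at a distance.
; A successful interact plays a 2D sound, increments the Key count on BP_ThirdPersonCharacter, prints it and destroys the actor.
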(event `self.ReceiveBeginPlay`
  ;[0.542 0.8687 1] interacion botiquin
  (`self.EnableInput` (`GameplayStatics.GetPlayerController` 0)))

(event `EnhancedInput|/Game/ThirdPerson/Input/Actions/IA_Interact`
  (params (ActionValue :type Boolean) (ElapsedSeconds :type "Float (double-precision)") (TriggeredSeconds :type "Float (double-precision)") (InputAction :type "InputAction Object Reference" :default "/Game/ThirdPerson/Input/Actions/IA_Interact.IA_Interact"))
  ;[0.542 0.8687 1] interacion botiquin
  (:`Started`
    ;;[1 0.9594 0.3846] Parra controlar el bug de que pueda coger-lo dedes cualquir parte ponemos este muro
    (`/Engine/EditorBlueprintResources/StandardMacros.Gate` true :!label _label
      (:`Exit`
        (`GameplayStatics.PlaySound2D` "/Game/MyAssets/Sonidos/PROPS/llave/SC_Llave.SC_Llave" 1.0 1.0 0.0 null null)
        (bind _asbp_third_person_character (cast `/Game/ThirdPerson/Blueprints/BP_ThirdPersonCharacter` (`GameplayStatics.GetPlayerCharacter` 0)))
        ;[1 1 1] Sumamos uno la varible de las llabes del personage
        (bind _result (`/Engine/EditorBlueprintResources/StandardMacros.IncrementInt` (`/Game/ThirdPerson/Blueprints/BP_ThirdPersonCharacter.Key` _asbp_third_person_character))
          (:`  `
            (`KismetSystemLibrary.PrintString` (`KismetStringLibrary.Conv_IntToString` _result))
            (`self.K2_DestroyActor`)))))))

(event `self.ReceiveActorBeginOverlap`
  (params (OtherActor :type "Actor Object Reference"))
  ;[0.542 0.8687 1] interacion botiquin
  ;;[0.4062 1 0.3229] si tocas el botiquin se abre el muro
  (goto _label :!via `Open`))

(event `self.ReceiveActorEndOverlap`
  (params (OtherActor :type "Actor Object Reference"))
  ;[0.542 0.8687 1] interacion botiquin
  ;;[1 0.3383 0.2785] cuando no tocas el botiquin se abre el muro
  (goto _label :!via `Close`))

(fn `UserConstructionScript`)