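; Rotatable judge statue for a puzzle, turned with the interact input while an actor overlaps it.
; A gate limits input to the overlap, and a DoOnce blocks repeat presses during rotation.
; Each press cycles Position through four quarter turns, animated by a timeline with shortest-path rotator lerp.
; At position zero it plays a success sound and updates the Sinner's puzzle after a delay, without re-arming interaction; other positions re-arm it.
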(event `self.ReceiveBeginPlay`
  ;[0.542 0.8687 1] interacion
  (`self.EnableInput` (`GameplayStatics.GetPlayerController` 0))
  (`self.ActivateAnimation`))

(event `EnhancedInput|/Game/ThirdPerson/Input/Actions/IA_Interact`
  (params (ActionValue :type Boolean) (ElapsedSeconds :type "Float (double-precision)") (TriggeredSeconds :type "Float (double-precision)") (InputAction :type "InputAction Object Reference" :default "/Game/ThirdPerson/Input/Actions/IA_Interact.IA_Interact"))
  ;[0.542 0.8687 1] interacion
  (:`Started`
    ;;[1 0.9594 0.3846] delimita el espacio de interacion
    (`/Engine/EditorBlueprintResources/StandardMacros.Gate` true :!label _label
      (:`Exit`
        (`/Engine/EditorBlueprintResources/StandardMacros.DoOnce` false :!label _label_2
          (:`Completed`
            (`self.UpdatePosition`)
            (`KismetSystemLibrary.PrintString` "Interacted")))))))

(event `InteracReset`
  (goto _label_2 :!via `Reset`))

(event `self.ReceiveActorBeginOverlap`
  (params (OtherActor :type "Actor Object Reference"))
  ;[0.542 0.8687 1] interacion
  (goto _label :!via `Open`))

(event `self.ReceiveActorEndOverlap`
  (params (OtherActor :type "Actor Object Reference"))
  ;[0.542 0.8687 1] interacion
  (goto _label :!via `Close`))

(event `UpdatePosition`
  ;[0.9217 0.3325 1] Cnvio de posicion, MAXIMO 3 si pasa del 3 vuelbe al 0
  (bind _result (`/Engine/EditorBlueprintResources/StandardMacros.IncrementInt` (`self.Position`))
    (:`  `
      (if (> _result 3)
        (set `self.Position` 0))
      (`self.ActivateAnimation`))))

(event `CheckPosition`
  ;[0.9224 1 0.1888] Comprobamos en que posicion esta la estatua
  (if (== (`self.Position`) 0)
    (`GameplayStatics.SpawnSoundAtLocation` "/Game/MyAssets/statues/Sound/statue_correctposition_Cue.statue_correctposition_Cue" (`self.K2_GetActorLocation`) (struct) 1.0 1.0 0.0 null null)
    (`KismetSystemLibrary.Delay` 0.75)
    (`/Game/MyAssets/statues/BP_Status_Sinner.UpdatePuzzle` (`self.Sinner`))
    (else
      (`self.InteracReset`))))

(event `ActivateAnimation`
  (set `self.StarRotation` (`self.EndRotation`))
  (set `self.EndRotation` (`KismetMathLibrary.MakeRotator` 0.0 0.0 (* (`self.Position`) 90.0)))
  (`GameplayStatics.SpawnSoundAtLocation` "/Game/MyAssets/statues/Sound/statue_rotate_Cue.statue_rotate_Cue" (`self.K2_GetActorLocation`) (struct) 1.0 1.0 0.0 null null)
  (bind (_direction _alpha) (`Timeline|Rotation` :!via `PlayFromStart`)
    (:`Update`
      (`SceneComponent.K2_SetRelativeRotation` (`self.Statue_Judge`) (`KismetMathLibrary.RLerp` (`self.StarRotation`) (`self.EndRotation`) _alpha true) false false))
    (:`Finished`
      (`self.CheckPosition`))))

(fn `UserConstructionScript`)