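; BP_Door is an interactable door that opens and closes, optionally locked behind a key carried by BP_ThirdPersonCharacter.
; Actor overlap opens and closes a Gate, so IA_Interact only works within range.
; A locked door consumes one key to unlock, or plays a locked sound and prints a warning.
; A FlipFlop plays or reverses a timeline that lerps yaw to ±90 degrees, chosen by Direcion, with sounds.
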(event `self.ReceiveBeginPlay`
  ;[0.542 0.8687 1] interacion botiquin
  (`self.EnableInput` (`GameplayStatics.GetPlayerController` 0))
  (bind _asbp_third_person_character (cast `/Game/ThirdPerson/Blueprints/BP_ThirdPersonCharacter` (`GameplayStatics.GetPlayerCharacter` 0)))
  (set `self.Character` _asbp_third_person_character)
  (if (`self.Direcion`)
    (set `self.DoorDirection` (struct :`Yaw` 90.0))
    (else
      (set `self.DoorDirection` (struct :`Yaw` -90.0)))))

(event `EnhancedInput|/Game/ThirdPerson/Input/Actions/IA_Interact`
  (params (ActionValue :type Boolean) (ElapsedSeconds :type "Float (double-precision)") (TriggeredSeconds :type "Float (double-precision)") (InputAction :type "InputAction Object Reference" :default "/Game/ThirdPerson/Input/Actions/IA_Interact.IA_Interact"))
  ;[0.542 0.8687 1] interacion botiquin
  (:`Started`
    ;;[1 0.9594 0.3846] Parra controlar el bug de que pueda coger el botiquin dedes cualquir parte ponemos este muro
    (`/Engine/EditorBlueprintResources/StandardMacros.Gate` true :!label _label
      (:`Exit`
        (if (`self.IsLocked?`)
          (if (>= (`/Game/ThirdPerson/Blueprints/BP_ThirdPersonCharacter.Key` (`self.Character`)) 1)
            (set `self.IsLocked?` false)
            (`GameplayStatics.PlaySound2D` "/Game/MyAssets/Sonidos/PROPS/Door/SC_Door_Unlock.SC_Door_Unlock" 1.0 1.0 0.0 null null)
            (`KismetSystemLibrary.Delay` 0.5)
            (`/Engine/EditorBlueprintResources/StandardMacros.DecrementInt` (`/Game/ThirdPerson/Blueprints/BP_ThirdPersonCharacter.Key` (`self.Character`))
              (:`  `
                (`self.OpenCloseDoor`)))
            (else
              (`GameplayStatics.PlaySound2D` "/Game/MyAssets/Sonidos/PROPS/Door/SC_Door_Locked.SC_Door_Locked" 1.0 1.0 0.0 null null)
              (`KismetSystemLibrary.PrintString` "NECESITAS UNA LLAVE!!")))
          (else
            (`self.OpenCloseDoor`)))))))

(event `self.ReceiveActorBeginOverlap`
  (params (OtherActor :type "Actor Object Reference"))
  ;[0.542 0.8687 1] interacion botiquin
  ;;[0.4062 1 0.3229] si tocas el botiquin se abre el muro
  (goto _label :!via `Open`))

(event `OpenCloseDoor`
  (`/Engine/EditorBlueprintResources/StandardMacros.FlipFlop`
    (:`A`
      (`GameplayStatics.PlaySound2D` "/Game/MyAssets/Sonidos/PROPS/Door/SC_Door_Open.SC_Door_Open" 1.0 1.0 0.0 null null)
      (bind (_direction _alpha) (`Timeline|door_rotation` :!label _label_2)
        (:`Update`
          (`SceneComponent.K2_SetRelativeRotation` (`self.Door_Door_GEO`) (`KismetMathLibrary.RLerp` (struct) (`self.DoorDirection`) _alpha) false false))))
    (:`B`
      (`GameplayStatics.PlaySound2D` "/Game/MyAssets/Sonidos/PROPS/Door/SC_Door_Close.SC_Door_Close" 1.0 1.0 0.0 null null)
      (goto _label_2 :!via `Reverse`))))

(event `self.ReceiveActorEndOverlap`
  (params (OtherActor :type "Actor Object Reference"))
  ;[0.542 0.8687 1] interacion botiquin
  ;;[1 0.3383 0.2785] cuando no tocas el botiquin se abre el muro
  (goto _label :!via `Close`))

(fn `UserConstructionScript`)