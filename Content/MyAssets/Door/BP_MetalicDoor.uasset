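; Metallic door Blueprint that swings open and closed with matching sounds each time its OpenCloseDoor event is called.
; BeginPlay uses the Direcion flag to choose which way the door turns by a quarter turn.
; A FlipFlop alternates between playing and reversing the Door_rotation timeline, whose alpha lerps the door mesh's relative rotation toward that target.
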(event `self.ReceiveBeginPlay`
  ;[0.542 0.8687 1] interacion botiquin
  ;;[1 1 1] Direcion de la puerta
  (if (`self.Direcion`)
    (set `self.DoorDirection` (struct :`Yaw` 90.0))
    (else
      (set `self.DoorDirection` (struct :`Yaw` -90.0)))))

(event `OpenCloseDoor`
  ;[0.9334 0.4583 1] Evento de cerar o abrir la puesta
  ;;[0.542 0.8687 1] interacion botiquin
  (`/Engine/EditorBlueprintResources/StandardMacros.FlipFlop`
    (:`A`
      (`GameplayStatics.PlaySound2D` "/Game/MyAssets/Sonidos/PROPS/Door/SC_Door_Open.SC_Door_Open" 1.0 1.0 0.0 null null)
      (bind (_direction _alpha) (`Timeline|door_rotation` :!label _label)
        (:`Update`
          (`SceneComponent.K2_SetRelativeRotation` (`self.Door_Door_GEO`) (`KismetMathLibrary.RLerp` (struct) (`self.DoorDirection`) _alpha) false false))))
    (:`B`
      (`GameplayStatics.PlaySound2D` "/Game/MyAssets/Sonidos/PROPS/Door/SC_Door_Close.SC_Door_Close" 1.0 1.0 0.0 null null)
      (goto _label :!via `Reverse`))))

(fn `UserConstructionScript`)