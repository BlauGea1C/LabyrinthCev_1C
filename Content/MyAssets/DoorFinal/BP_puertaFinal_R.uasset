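; BP_puertaFinal_R is a final double door that slides open once its lever counter runs out.
; Each PuertaFinal call decrements NumPalancas; at zero or below, a short delay precedes the DoorFinalAnimation timeline.
; That timeline moves SMFinalDoorR and, from its update, plays a second timeline that moves SMFinalDoor.
; Overlap opens and closes a gate on the interact input, but the gate's exit drives nothing.
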(event `self.ReceiveBeginPlay`
  (`self.EnableInput` (`GameplayStatics.GetPlayerController` 0)))

(event `PuertaFinal`
  (bind _result (`/Engine/EditorBlueprintResources/StandardMacros.DecrementInt` (`self.NumPalancas`))
    (:`  `
      (if (<= _result 0)
        (`KismetSystemLibrary.Delay` 0.4)
        (bind (_direction _alpha) (`Timeline|DoorFinalAnimation`)
          (:`Update`
            (`SceneComponent.K2_SetRelativeLocation` (`self.SM_FinalDoor_R`) (`KismetMathLibrary.VLerp` (-224.0 0.0 0.0) (-425.0 0.0 0.0) _alpha) false false)
            (bind (_direction_2 _alpha_2) (`Timeline|Timeline`)
              (:`Update`
                (`SceneComponent.K2_SetRelativeLocation` (`self.SM_FinalDoor`) (`KismetMathLibrary.VLerp` (270.0 0.0 0.0) (530.0 0.0 0.0) _alpha_2) false false)))))))))

(event `EnhancedInput|/Game/ThirdPerson/Input/Actions/IA_Interact`
  (params (ActionValue :type Boolean) (ElapsedSeconds :type "Float (double-precision)") (TriggeredSeconds :type "Float (double-precision)") (InputAction :type "InputAction Object Reference" :default "/Game/ThirdPerson/Input/Actions/IA_Interact.IA_Interact"))
  (:`Started`
    (`/Engine/EditorBlueprintResources/StandardMacros.Gate` true :!label _label)))

(event `self.ReceiveActorBeginOverlap`
  (params (OtherActor :type "Actor Object Reference"))
  (goto _label :!via `Open`))

(event `self.ReceiveActorEndOverlap`
  (params (OtherActor :type "Actor Object Reference"))
  (goto _label :!via `Close`))

(fn `UserConstructionScript`)