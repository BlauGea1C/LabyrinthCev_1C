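; Demogorgon enemy character that roams near the player, then screams, chases and attacks once it spots them.
; Blueprint events form the AI loop through AIMoveTo and PawnSensing, with a retriggerable delay returning it to roaming after lost sight.
; Reaching a player who plays dead triggers roaming; otherwise it plays random attack montages, while AttackTrail applies damage via forward sphere trace.
; Rear detection and Bounce events are empty.
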(event `self.ReceiveBeginPlay`
  (bind _asbp_third_person_character (cast `/Game/ThirdPerson/Blueprints/BP_ThirdPersonCharacter` (`GameplayStatics.GetPlayerCharacter` 0)))
  (set `self.PlayerCharacter` _asbp_third_person_character)
  (`self.Roam`))

(event `Roam`
  (`GameplayStatics.PlaySound2D` "/Game/MyAssets/Sonidos/Demogorgon/SC_idel_demo.SC_idel_demo" 1.0 1.0 0.0 null null)
  (set `CharacterMovementComponent.MaxWalkSpeed` (`self.SpeedRoam`) (`self.CharacterMovement`))
  (bind _randomlocation (`NavigationSystemV1.K2_GetRandomLocationInNavigableRadius` (`self.K2_GetActorLocation` (`self.PlayerCharacter`)) 2500.0 null null))
  (`|AIMoveTo` self _randomlocation null 150.0
    (:`OnSuccess`
      (`KismetSystemLibrary.Delay` (`KismetMathLibrary.RandomFloatInRange` 2.0 8.0))
      (if (not (`self.IsChasing`))
        (`self.Roam`)))))

(event `TryNotSeePawn`
  (`KismetSystemLibrary.RetriggerableDelay` 5.0)
  (set `self.IsChasing` false)
  (`self.AlertReset`)
  (`self.Stop`)
  (`KismetSystemLibrary.Delay` (`KismetMathLibrary.RandomFloatInRange` 1.0 3.0))
  (if (not (`self.IsChasing`))
    (`self.Roam`)))

(event `self.PawnSensing.OnSeePawn`
  (params (Pawn :type "Pawn Object Reference"))
  (if (== Pawn (`self.PlayerCharacter`))
    (`self.TryNotSeePawn`)
    (`/Engine/EditorBlueprintResources/StandardMacros.DoOnce` false :!label _label
      (:`Completed`
        (`self.Alert`)))))

(event `AlertReset`
  (goto _label :!via `Reset`))

(event `self.RearDetection.OnComponentBeginOverlap`
  (params (OverlappedComponent :type "PrimitiveComponent Object Reference") (OtherActor :type "Actor Object Reference") (OtherComp :type "PrimitiveComponent Object Reference") (OtherBodyIndex :type Integer) (bFromSweep :type Boolean) (SweepResult :type "HitResult Structure (by ref)")))

(event `Alert`
  (`self.Stop`)
  (set `self.IsChasing` true)
  (set `CharacterMovementComponent.MaxWalkSpeed` (`self.SpeedChase`) (`self.CharacterMovement`))
  (`GameplayStatics.SpawnSoundAtLocation` "/Game/Characters/Demogorgon/Sonidos/SC_gritoDemogorgon.SC_gritoDemogorgon" (`self.K2_GetActorLocation`) (struct) 1.0 1.0 0.0 null null)
  (bind _returnvalue (`self.PlayAnimMontage` "/Game/Characters/Demogorgon/Animation/AM_DemogorgonAlerta.AM_DemogorgonAlerta"))
  (`KismetSystemLibrary.Delay` _returnvalue)
  (`self.Chase`))

(event `Chase`
  (set `self.IsChasing` true)
  (`|AIMoveTo` self (0.0 0.0 0.0) (`self.PlayerCharacter`) 150.0
    (:`OnSuccess`
      (if (`/Game/ThirdPerson/Blueprints/BP_ThirdPersonCharacter.PlayDead` (`self.PlayerCharacter`))
        (`self.Roam`)
        (else
          (`self.Attack`)
          (`self.Chase`))))
    (:`OnFail`
      (if (`self.IsChasing`)
        (`self.Chase`)
        (`GameplayStatics.PlaySound2D` "/Game/MyAssets/Sonidos/Demogorgon/SC_Chase_demo.SC_Chase_demo" 1.0 1.0 0.0 null null)))))

(event `Stop`
  (`|AIMoveTo` self (0.0 0.0 0.0) self))

(event `Attack`
  (`/Engine/EditorBlueprintResources/StandardMacros.DoOnce` false :!label _label_2
    (:`Completed`
      (`GameplayStatics.PlaySound2D` "/Game/MyAssets/Sonidos/Demogorgon/SC_Attack_demo.SC_Attack_demo" 1.0 1.0 0.0 null null)
      (bind _returnvalue (`self.PlayAnimMontage` (`|GetArrayItem` (`self.AttackAnimations`) (`KismetMathLibrary.RandomIntegerInRange` 0 2))))
      (`KismetSystemLibrary.Delay` _returnvalue)
      (`self.AtackReset`)
      (`self.Chase`))))

(event `AtackReset`
  (goto _label_2 :!via `Reset`))

(event `Bounce`)

(event `AttackTrail`
  (bind _returnvalue (`self.K2_GetActorLocation`))
  (bind _outhit (`KismetSystemLibrary.SphereTraceSingle` :`Start` _returnvalue :`End` (+ _returnvalue (* (`self.GetActorForwardVector`) 250.0)) :`Radius` 50.0 :`TraceChannel` "TraceTypeQuery1" :`DrawDebugType` "Persistent"))
  (if (== (`.HitActor` (`GameplayStatics.BreakHitResult` _outhit)) (`self.PlayerCharacter`))
    (`/Game/ThirdPerson/Blueprints/BP_ThirdPersonCharacter.HealthManager` (`self.PlayerCharacter`) -30.0)))

(fn `UserConstructionScript`)